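; Enemy spawner that keeps up to four BP_Enemy AI pawns alive around the player.
; Every tick it jumps to a random distance along the camera's forward direction from the player pawn, rotated toward the player.
; While EnemyList is short, a randomized Delay on Tick leads to Generate, which spawns an enemy with BT_Enemy above the spawner.
; Each enemy receives a Generator reference; RemoveEnemy frees its slot.
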(event EventBeginPlay)

(event Collision|EventActorBeginOverlap
  (params (OtherActor :type Actor%20Object%20Reference)))

(event EventTick
  (params (DeltaSeconds :type Float%20%28single-precision%29))
  (bind _returnvalue (Game|Player|GetPlayerPawn 0))
  (bind _returnvalue_2 (Game|GetPlayerCameraManager 0))
  (bind _returnvalue_3 (Math|Random|RandomFloatinRange 6e+02 1.2e+03))
  (bind _returnvalue_4 (Transformation|GetActorTransform _returnvalue))
  (bind _returnvalue_5 (Transformation|GetActorForwardVector _returnvalue_2))
  (bind _location (Math|Transform|BreakTransform _returnvalue_4))
  (bind (_x _y) (Math|Vector|BreakVector _returnvalue_5))
  (bind (_x_2 _y_2 _z) (Math|Vector|BreakVector _location))
  (Transformation|SetActorTransform (Math|Transform|MakeTransform (Math|Vector|MakeVector (+ (* _returnvalue_3 _x) _x_2) (+ (* _returnvalue_3 _y) _y_2) _z) (Math|Conversions|RotationFromXVector (- _location (.Location (Math|Transform|BreakTransform (Transformation|GetActorTransform)))))))
  (if (< (Utilities|Array|Length (Variables|Default|GetEnemyList)) 4)
    (Utilities|FlowControl|Delay (Math|Random|RandomFloatinRange 3.0 7.0))
    (CallFunction|Generate)))

(fn ConstructionScript)

(fn Generate
  (bind _returnvalue (Transformation|GetActorTransform))
  (bind (_location _rotation) (Math|Transform|BreakTransform _returnvalue))
  (bind (_x _y _z) (Math|Vector|BreakVector _location))
  (bind _returnvalue_2 (AI|SpawnAIFromClass "/Game/Blueprints/BP_Enemy.BP_Enemy_C" "/Game/AI/BT_Enemy.BT_Enemy" (Math|Vector|MakeVector _x _y (+ _z 1.8e+02)) _rotation false 0))
  (bind _asbp_enemy (Utilities|Casting|CastToBP_Enemy _returnvalue_2))
  (Variables|/Game/Blueprints/BP_Enemy.BP_Enemy_C|SetGenerator _asbp_enemy self)
  (Utilities|Array|Add (Variables|Default|GetEnemyList) _returnvalue_2))

(fn RemoveEnemy
  (params (RemoveOne :type Actor%20Object%20Reference))
  (Utilities|Array|RemoveItem (Variables|Default|GetEnemyList) RemoveOne))