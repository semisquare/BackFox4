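; BP_AirDoor is a two-piece door that starts with no meshes and turns to stone after the player leaves its trigger volume.
; BeginPlay clears the static meshes on Door1 and Door2.
; When an actor tagged Player ends overlap with the Box, each piece receives its own stone mesh.
; Nothing in the graph clears the meshes again after that.
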(event OnComponentEndOverlap(Box)
  (params (OverlappedComponent :type Primitive%20Component%20Object%20Reference) (OtherActor :type Actor%20Object%20Reference) (OtherComp :type Primitive%20Component%20Object%20Reference) (OtherBodyIndex :type Integer))
  (if (Actor|ActorHasTag OtherActor "Player")
    (Components|StaticMesh|SetStaticMesh (Variables|Default|GetDoor1) "/Game/Assets/VoxelArch/SM_Stone_1.SM_Stone_1")
    (Components|StaticMesh|SetStaticMesh (Variables|Default|GetDoor2) "/Game/Assets/VoxelArch/SM_Stone_2.SM_Stone_2")))

(event EventBeginPlay
  (Components|StaticMesh|SetStaticMesh (Variables|Default|GetDoor1) 0)
  (Components|StaticMesh|SetStaticMesh (Variables|Default|GetDoor2) 0))

(event Collision|EventActorBeginOverlap
  (params (OtherActor :type Actor%20Object%20Reference)))

(event EventTick
  (params (DeltaSeconds :type Float%20%28single-precision%29)))

(fn ConstructionScript)