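; BP_Player is the player Blueprint, with very little active logic of its own.
; On BeginPlay it sets the DissolveRate scalar in the MPC_FJ material parameter collection to 1.
; Tick and ChangeWeapon are empty.
; Disconnected, unused nodes remain for depth of field focused at spring arm length, player UI creation and a stamina debug print.
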(event Custom|ChangeWeapon)

(event EventBeginPlay
  (Rendering|Material|SetScalarParameterValue "/Game/Materials/MPC_FJ.MPC_FJ" "DissolveRate" 1.0 :!class /Script/Engine.KismetMaterialLibrary))

(event Collision|EventActorBeginOverlap
  (params (OtherActor :type Actor%20Object%20Reference)))

(event EventTick
  (params (DeltaSeconds :type Float%20%28single-precision%29)))

(fn ConstructionScript)