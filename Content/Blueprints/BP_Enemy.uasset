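; BP_Enemy is an enemy character that displays combat UI and reports its death to the generator that tracks it.
; It attaches its CharacterUI widget to itself on BeginPlay and spawns floating damage text through the OnAttacked event.
; Pawn sensing lazily creates a viewport health widget, and AttributeComponent's death event removes the enemy from BP_GenerateEnemy.
; UpdateWalkSpeed sets movement speed, while a random-scale snippet is left unconnected.
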(event InDeath(AttributeComponent)
  (params (InstigatorActor :type Actor%20Object%20Reference) (OwingComp :type J%20Attribute%20Component%20Object%20Reference))
  (bind _asbp_generate_enemy (Utilities|Casting|CastToBP_GenerateEnemy (Variables|Default|GetGenerator)))
  (Default|RemoveEnemy _asbp_generate_enemy self))

(event OnSeePawn(PawnSensingComponent)
  (params (Pawn :type Pawn%20Object%20Reference))
  (Utilities|IsValid (Variables|Default|GetHealth)
    (:Is%20Not%20Valid
      (bind _returnvalue (UserInterface|CreateWidget "/Game/UI/WBP_EnemyHealth.WBP_EnemyHealth_C" 0 self))
      (bind _output_get (Variables|Default|SetHealth _returnvalue))
      (UserInterface|Viewport|AddtoViewport _output_get 0))))

(event Custom|OnAttacked_Event
  (params (InstigatorActor :type Actor%20Object%20Reference) (Damage :type Float%20%28single-precision%29))
  (bind _returnvalue (UserInterface|CreateWidget "/Game/UI/WBP_FloatText.WBP_FloatText_C" 0 self (Utilities|Text|ToText(Float) Damage "HalfToEven")))
  (UserInterface|Viewport|AddtoViewport _returnvalue 0))

(event EventBeginPlay
  (EventDispatchers|BindEventtoOnAttacked (delegate Custom|OnAttacked_Event))
  (bind _aswbp_enemy_ui (Utilities|Casting|CastToWBP_EnemyUI (UserInterface|GetUserWidgetObject (Variables|Default|GetCharacterUI))))
  (Variables|/Game/UI/WBP_EnemyUI.WBP_EnemyUI_C|SetAttachTo _aswbp_enemy_ui self))

(event Collision|EventActorBeginOverlap
  (params (OtherActor :type Actor%20Object%20Reference)))

(event EventTick
  (params (DeltaSeconds :type Float%20%28single-precision%29)))

(fn ConstructionScript)

(fn UpdateWalkSpeed
  (params (Speed :type Float%20%28double-precision%29))
  (Variables|/Script/Engine.CharacterMovementComponent|SetMaxWalkSpeed (Variables|Character|GetCharacterMovement) Speed))